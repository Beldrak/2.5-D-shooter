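; Shotgun weapon Blueprint that fires and plays a sprite flipbook animation when ShootWeapon is called.
; ShootWeapon checks for enough ammo, then passes a DoOnce gate to decrease ammo, call FireWeapon and play the fire flipbook.
; A delay matching that flipbook's length returns it to idle and calls Resetfire, which reopens the gate, so the animation length sets the fire rate.
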(event `self.ShootWeapon`
  (bind _weaponflipbook (`self.Weaponflipbook`))
  (bind _hasammo (`self.Has Enough Ammo?`))
  (if _hasammo
    (`/Engine/EditorBlueprintResources/StandardMacros.DoOnce` false :!label _label
      (:`Completed`
        (`self.DecreaseAmmo`)
        (`self.FireWeapon`)
        (`PaperFlipbookComponent.SetFlipbook` _weaponflipbook "/Game/RetroFPSAssets/Weapons/Shotgun/ShotGunFire.ShotGunFire")
        (`KismetSystemLibrary.Delay` (`PaperFlipbookComponent.GetFlipbookLength` _weaponflipbook))
        (`PaperFlipbookComponent.SetFlipbook` (`self.Weaponflipbook`) "/Game/RetroFPSAssets/Weapons/Shotgun/ShotGunIdle.ShotGunIdle")
        (`self.Resetfire`)))))

(event `Resetfire`
  (goto _label :!via `Reset`))

(fn `UserConstructionScript`
  (`parent.UserConstructionScript`))