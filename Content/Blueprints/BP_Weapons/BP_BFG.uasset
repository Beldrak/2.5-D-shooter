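; BP_BFG is the BFG weapon Blueprint, a flipbook-animated gun that fires a projectile using the player's Cell ammo.
; ShootWeapon requires enough cells for a shot and uses a DoOnce gate to block re-firing mid-shot.
; It plays the fire flipbook, delays for that animation's length, then calls FireProjectile and returns to idle.
; It then deducts the cells, refreshes the HUD ammo display and resets the gate via RESETDOONCE.
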(event `self.ShootWeapon`
  (bind _playercharacter (`self.PlayerCharacter`))
  (bind _weaponflipbook (`self.Weaponflipbook`))
  (if (>= (`/Game/FirstPerson/Blueprints/BP_FirstPersonCharacter.Cell` (`self.PlayerCharacter`)) 30)
    (`/Engine/EditorBlueprintResources/StandardMacros.DoOnce` false :!label _label
      (:`Completed`
        (`PaperFlipbookComponent.SetFlipbook` _weaponflipbook "/Game/RetroFPSAssets/Weapons/BFG/BFGFire.BFGFire")
        (`KismetSystemLibrary.Delay` (`PaperFlipbookComponent.GetFlipbookLength` _weaponflipbook))
        (`self.FireProjectile`)
        (`PaperFlipbookComponent.SetFlipbook` (`self.Weaponflipbook`) "/Game/RetroFPSAssets/Weapons/BFG/BFGIdle.BFGIdle")
        (set `/Game/FirstPerson/Blueprints/BP_FirstPersonCharacter.Cell` (- (`/Game/FirstPerson/Blueprints/BP_FirstPersonCharacter.Cell` _playercharacter) 30) _playercharacter)
        (`/Game/Blueprints/UI/PlayerHUD.UpdateCellammo` (`/Game/FirstPerson/Blueprints/BP_FirstPersonCharacter.PlayerHUD` _playercharacter))
        (`self.RESETDOONCE`)))))

(event `RESETDOONCE`
  (goto _label :!via `Reset`))

(fn `UserConstructionScript`
  (`parent.UserConstructionScript`))