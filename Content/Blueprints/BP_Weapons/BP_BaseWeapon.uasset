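; Base weapon Blueprint providing hitscan and projectile firing plus typed ammo handling, with empty shoot and stop events.
; FireWeapon line-traces from a component, with debug drawing, and applies damage on hit.
; FireProjectile spawns a projectile carrying speed and damage.
; Ammo checks and decrements use the player character's Bullet, Shell, Rocket or Cell counts through a reference cached on BeginPlay, updating the HUD after use.
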(event `DecreaseAmmo`
  ;[1 1 1] Use Ammo function // double click Use Ammo to see the code
  (`self.UseAmmo`))

(event `self.ReceiveBeginPlay`
  ;[1 1 1] We are creating a character refrence on the begin play, so we don't have to cast everywhere here.
  (bind _asbp_first_person_character (cast `/Game/FirstPerson/Blueprints/BP_FirstPersonCharacter` (`GameplayStatics.GetPlayerCharacter` 0)))
  (set `self.PlayerCharacter` _asbp_first_person_character))

(event `ShootWeapon`)

(event `StopShooting`)

(fn `FireProjectile`
  (`|SpawnActorFromClass` (`self.Projectile`) (`SceneComponent.K2_GetComponentToWorld` (`self.ProjectileTransform`)) "Undefined" "MultiplyWithRoot" null (`self.ProjectileSpeed`) (`self.Weapon Damage`) null))

(fn `FireWeapon`
  (bind _returnvalue (`SceneComponent.K2_GetComponentLocation` (`self.linetrace`)))
  (bind (_outhit _returnvalue_2) (`KismetSystemLibrary.LineTraceSingleForObjects` _returnvalue (+ _returnvalue (* (`KismetMathLibrary.GetForwardVector` (`SceneComponent.K2_GetComponentRotation` (`self.linetrace`))) (`self.linetraceDistance`))) (`|MakeArray` "ObjectTypeQuery1" "ObjectTypeQuery2" "ObjectTypeQuery3" :!type "EObjectTypeQuery Enum") false (`|MakeArray` self (`GameplayStatics.GetPlayerCharacter` 0) :!type "Actor Object Reference") "ForDuration"))
  (if _returnvalue_2
    ;[1 0.09896 0.09896] Weapon Damage changes with what weapon is being used. Do not change the value here
    (`GameplayStatics.ApplyDamage` (`.HitActor` (`GameplayStatics.BreakHitResult` _outhit)) (`self.Weapon Damage`))))

(fn `Has Enough Ammo?`
  (returns (HasAmmo :type Boolean))
  (bind _playercharacter (`self.PlayerCharacter`))
  (switch `/Game/Blueprints/BP_Weapons/Ammo` (`self.AmmoType`)
    (:`NewEnumerator0`
      (if (> (`/Game/FirstPerson/Blueprints/BP_FirstPersonCharacter.Bullet` _playercharacter) 0)
        (return true)
        (else
          (return false))))
    (:`NewEnumerator1`
      (if (> (`/Game/FirstPerson/Blueprints/BP_FirstPersonCharacter.Shell` _playercharacter) 0)
        (return true)
        (else
          (return false))))
    (:`NewEnumerator2`
      (if (> (`/Game/FirstPerson/Blueprints/BP_FirstPersonCharacter.Rocket` _playercharacter) 0)
        (return true)
        (else
          (return false))))
    (:`NewEnumerator3`
      (if (> (`/Game/FirstPerson/Blueprints/BP_FirstPersonCharacter.Cell` _playercharacter) 0)
        (return true)
        (else
          (return false))))))

(fn `UseAmmo`
  (bind _playercharacter (`self.PlayerCharacter`))
  (bind _playerhud (`/Game/FirstPerson/Blueprints/BP_FirstPersonCharacter.PlayerHUD` _playercharacter))
  (switch `/Game/Blueprints/BP_Weapons/Ammo` (`self.AmmoType`)
    (:`NewEnumerator0`
      (`/Engine/EditorBlueprintResources/StandardMacros.DecrementInt` (`/Game/FirstPerson/Blueprints/BP_FirstPersonCharacter.Bullet` _playercharacter)
        (:`  `
          (`/Game/Blueprints/UI/PlayerHUD.UpdateBulletAmmo` _playerhud))))
    (:`NewEnumerator1`
      (`/Engine/EditorBlueprintResources/StandardMacros.DecrementInt` (`/Game/FirstPerson/Blueprints/BP_FirstPersonCharacter.Shell` _playercharacter)
        (:`  `
          (`/Game/Blueprints/UI/PlayerHUD.UpdateShellAmmo` _playerhud))))
    (:`NewEnumerator2`
      (`/Engine/EditorBlueprintResources/StandardMacros.DecrementInt` (`/Game/FirstPerson/Blueprints/BP_FirstPersonCharacter.Rocket` _playercharacter)
        (:`  `
          (`/Game/Blueprints/UI/PlayerHUD.UpdateRocketAmmo` _playerhud))))
    (:`NewEnumerator3`
      (`/Engine/EditorBlueprintResources/StandardMacros.DecrementInt` (`/Game/FirstPerson/Blueprints/BP_FirstPersonCharacter.Cell` _playercharacter)
        (:`  `
          (`/Game/Blueprints/UI/PlayerHUD.UpdateCellammo` _playerhud))))))

(fn `UserConstructionScript`)