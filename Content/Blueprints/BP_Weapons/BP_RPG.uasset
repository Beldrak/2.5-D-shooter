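; BP_RPG is a rocket launcher weapon that fires a projectile and animates with Paper2D flipbooks.
; ShootWeapon checks ammo, then passes a DoOnce gate to decrease ammo, fire and switch the flipbook from idle to fire.
; After the fire flipbook's length it returns to idle, waits a fixed cooldown, then calls ResetWeapon to reopen the gate.
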(event `self.ShootWeapon`
  (bind _weaponflipbook (`self.Weaponflipbook`))
  (bind _hasammo (`self.Has Enough Ammo?`))
  (if _hasammo
    (`/Engine/EditorBlueprintResources/StandardMacros.DoOnce` false :!label _label
      (:`Completed`
        (`self.DecreaseAmmo`)
        (`self.FireProjectile`)
        (`PaperFlipbookComponent.SetFlipbook` _weaponflipbook "/Game/RetroFPSAssets/Weapons/RPG/RPGFire.RPGFire")
        (`KismetSystemLibrary.Delay` (`PaperFlipbookComponent.GetFlipbookLength` _weaponflipbook))
        (`PaperFlipbookComponent.SetFlipbook` (`self.Weaponflipbook`) "/Game/RetroFPSAssets/Weapons/RPG/RPGIdle.RPGIdle")
        (`KismetSystemLibrary.Delay` 2.0)
        (`self.ResetWeapon`)))))

(event `ResetWeapon`
  (goto _label :!via `Reset`))

(fn `UserConstructionScript`
  (`parent.UserConstructionScript`))