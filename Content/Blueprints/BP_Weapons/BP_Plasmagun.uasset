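; Plasma gun weapon Blueprint that fires projectiles automatically and animates with Paper2D flipbooks.
; ShootWeapon starts a looping timer through a DoOnce gate; each tick checks ammo, spends it, fires a projectile and shows the firing flipbook.
; StopShooting clears the timer, restores the idle flipbook and resets the gate.
; An empty-ammo tick also restores idle and resets the gate, but leaves the timer running.
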(event `self.ShootWeapon`
  (`/Engine/EditorBlueprintResources/StandardMacros.DoOnce` false :!label _label
    (:`Completed`
      (bind _returnvalue (`KismetSystemLibrary.K2_SetTimerDelegate` (delegate `FireMiniGun`) 0.15 true))
      (set `self.MiniGunEvent` _returnvalue))))

(event `Resetfire`
  (goto _label :!via `Reset`))

(event `FireMiniGun`
  (bind _hasammo (`self.Has Enough Ammo?`))
  (if _hasammo
    (`self.DecreaseAmmo`)
    (`self.FireProjectile`)
    (`PaperFlipbookComponent.SetFlipbook` (`self.Weaponflipbook`) "/Game/RetroFPSAssets/Weapons/PlasmaGun/PlasmaFire.PlasmaFire")
    (else
      (`PaperFlipbookComponent.SetFlipbook` (`self.Weaponflipbook`) "/Game/RetroFPSAssets/Weapons/PlasmaGun/PlasmaIdle.PlasmaIdle" :!label _label_2)
      (`self.Resetfire`))))

(event `self.StopShooting`
  (`KismetSystemLibrary.K2_ClearAndInvalidateTimerHandle` (`self.MiniGunEvent`))
  (goto _label_2))

(fn `UserConstructionScript`
  (`parent.UserConstructionScript`))