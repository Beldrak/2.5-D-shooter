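; Weapon pickup actor that shows a 2D Paper sprite and grants a weapon to the first-person character that touches it.
; The construction script maps the Weapon enum to a sprite and weapon class, with RPG currently assigned the Plasmagun class.
; Tick billboards the actor by yawing it toward the player.
; Sphere overlap passes the class to the character's PickupWeapon, then destroys the pickup.
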(event `self.ReceiveTick`
  (params (DeltaSeconds :type "Float (single-precision)"))
  (bind (_returnvalue_roll _returnvalue_pitch _returnvalue_yaw) (`KismetMathLibrary.BreakRotator` (`KismetMathLibrary.FindLookAtRotation` (`self.K2_GetActorLocation`) (`self.K2_GetActorLocation` (`GameplayStatics.GetPlayerCharacter` 0)))))
  ;[1 1 1] Always making sure the weapon sprite is facing the players current location
  (`self.K2_SetActorRotation` (`KismetMathLibrary.MakeRotator` 0.0 0.0 _returnvalue_yaw)))

(event `self.Sphere.OnComponentBeginOverlap`
  (params (OverlappedComponent :type "PrimitiveComponent Object Reference") (OtherActor :type "Actor Object Reference") (OtherComp :type "PrimitiveComponent Object Reference") (OtherBodyIndex :type Integer) (bFromSweep :type Boolean) (SweepResult :type "HitResult Structure (by ref)"))
  ;[1 1 1] Player Overlaps->Pick up Weapon
  (bind _asbp_first_person_character (cast `/Game/FirstPerson/Blueprints/BP_FirstPersonCharacter` OtherActor))
  (`/Game/FirstPerson/Blueprints/BP_FirstPersonCharacter.PickupWeapon` _asbp_first_person_character (`self.WeaponClass`))
  (`self.K2_DestroyActor`))

(fn `UserConstructionScript`
  (bind _papersprite (`self.PaperSprite`))
  (switch `/Game/Blueprints/BP_Weapons/WeaponPickUpSystem/Weapon` (`self.Weapon`)
    (:`NewEnumerator0`
      (`PaperSpriteComponent.SetSprite` _papersprite "/Game/RetroFPSAssets/Weapons/Shotgun/ShotgunSprite.ShotgunSprite")
      (set `self.WeaponClass` "/Game/Blueprints/BP_Weapons/BP_Shotgun.BP_Shotgun_C"))
    (:`NewEnumerator1`
      (`PaperSpriteComponent.SetSprite` _papersprite "/Game/RetroFPSAssets/Weapons/MiniGun/minigunsprite.minigunsprite")
      (set `self.WeaponClass` "/Game/Blueprints/BP_Weapons/BP_MiniGun.BP_MiniGun_C"))
    (:`NewEnumerator2`
      (`PaperSpriteComponent.SetSprite` _papersprite "/Game/RetroFPSAssets/Weapons/PlasmaGun/PlasmaSprite.PlasmaSprite")
      (set `self.WeaponClass` "/Game/Blueprints/BP_Weapons/BP_Plasmagun.BP_Plasmagun_C"))
    (:`NewEnumerator3`
      (`PaperSpriteComponent.SetSprite` _papersprite "/Game/RetroFPSAssets/Weapons/RPG/RPGSprite.RPGSprite")
      (set `self.WeaponClass` "/Game/Blueprints/BP_Weapons/BP_Plasmagun.BP_Plasmagun_C"))
    (:`NewEnumerator4`
      (`PaperSpriteComponent.SetSprite` _papersprite "/Game/RetroFPSAssets/Weapons/BFG/BFGSprite.BFGSprite")
      (set `self.WeaponClass` "/Game/Blueprints/BP_Weapons/BP_BFG.BP_BFG_C"))
    (:`NewEnumerator5`
      (`PaperSpriteComponent.SetSprite` _papersprite "/Game/RetroFPSAssets/Weapons/Chainsaw/ChainsawSprite.ChainsawSprite")
      (set `self.WeaponClass` "/Game/Blueprints/BP_Weapons/BP_Chainsaw.BP_Chainsaw_C"))))